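; Player controller for a networked twin-stick character with touch joysticks: left stick moves, right stick turns the pawn.
; Right-stick input is relayed via server events, toggling orient-to-movement against controller yaw and lerping FaceRotation, whose OnRep sets control rotation.
; A TurnInPlace macro compares delayed yaw and axis samples to drive the character's turn state.
; BeginPlay spawns an M4 on the mesh socket; Fire presses it, stick release releases it.
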(event Custom|StickRotatorServer
  (params (X :type Float%20%28single-precision%29) (Y :type Float%20%28single-precision%29))
  ;[1 1 1] Replicate To Server
  (CallFunction|StickRotatorAll X Y))

(event Custom|SRV_SnapWeapon
  ;[1 1 1] Protected
  (CallFunction|SnapWeapon))

(event Custom|Covered
  (params (Movement :type Character%20Movement%20Component%20Object%20Reference) (Yaw :type Pawn%20Object%20Reference))
  ;[1 1 1] RightStick Covered or Not covered
  (Variables|/Script/Engine.CharacterMovementComponent|SetbOrientRotationToMovement Movement false)
  (Variables|/Script/Engine.Pawn|SetbUseControllerRotationYaw Yaw true)
  (CallFunction|RotateNow))

(event Custom|NotCovered
  (params (Char%20Movement%20F :type Character%20Movement%20Component%20Object%20Reference) (Character%20F :type Pawn%20Object%20Reference))
  ;[1 1 1] RightStick Covered or Not covered
  (Variables|/Script/Engine.CharacterMovementComponent|SetbOrientRotationToMovement Char%20Movement%20F true)
  (Variables|/Script/Engine.Pawn|SetbUseControllerRotationYaw Character%20F false))

(event Custom|StickRotatorAll
  (params (X :type Float%20%28single-precision%29) (Y :type Float%20%28single-precision%29))
  (bind _returnvalue (Pawn|GetControlledPawn))
  (bind _returnvalue_2 (Math|Vector|MakeVector X Y 0.0))
  (bind _returnvalue_3 (Math|Vector|VectorLength _returnvalue_2))
  ;[1 1 1] RightStick
  (bind _ascharacter_bp (Utilities|Casting|CastToCharacter_BP _returnvalue))
  (Variables|Default|SetAxis _returnvalue_3)
  (bind _output_get (Variables|Default|SetIsCovered? (!= _returnvalue_3 0.0)))
  (if _output_get
    (Utilities|FlowControl|Sequence
      (:then_0
        (CallFunction|Covered (Variables|/Script/Engine.Character|GetCharacterMovement _ascharacter_bp) _ascharacter_bp)
        (|TurnInPlace _ascharacter_bp (.yaw (Transformation|GetActorRotation _returnvalue)) :!label _label)))
    (else
      (Utilities|FlowControl|Sequence
        (:then_0
          (CallFunction|NotCovered (Variables|/Script/Engine.Character|GetCharacterMovement _ascharacter_bp) _ascharacter_bp)
          (goto _label NotCovered))
        (:then_1
          (Default|FireRealese (Variables|Default|GetNewVar_0)))))))

(event Custom|RotateNow
  (bind _returnvalue (Pawn|GetControlledPawn))
  (bind _returnvalue_2 (Transformation|GetActorLocation _returnvalue))
  ;[1 1 1] RightStick
  (Variables|Default|SetFaceRotation (Math|Rotator|Lerp(Rotator) (Math|Rotator|FindLookatRotation _returnvalue_2 (+ (Math|Vector|MakeVector (stale Custom|StickRotatorAll X) (stale Custom|StickRotatorAll Y) 0.0) _returnvalue_2)) (Transformation|GetActorRotation _returnvalue) 0.75 true)))

(event EventBeginPlay
  ;[1 0.1442 0.194] BeginPlay
  (Class|PlayerController|ActivateTouchInterface "/Engine/MobileResources/HUD/DefaultVirtualJoysticks.DefaultVirtualJoysticks")
  (Class|PlayerController|SetVirtualJoystickVisibility true)
  (CallFunction|SRVSnapWeapon)
  (Utilities|FlowControl|Sequence
    (:then_1
      ;[0 0 0] Dev
      (Networking|SwitchHasAuthority
        (:Authority
          (Development|PrintString "Server"))
        (:Remote
          (Development|PrintString "Client"))))
    (:then_2
      (Variables|Default|SetbShowMouseCursor true))))

(event Input|ActionEvents|InputActionFire
  (params (Key :type Key%20Structure))
  (:Pressed
    (Default|FirePress (Variables|Default|GetNewVar_0))))

(event Input|AxisEvents|InputAxisTurnRight
  (params (AxisValue :type Float%20%28single-precision%29))
  ;[1 1 1] RightStick
  (CallFunction|StickRotatorServer (/ (stale Input|AxisEvents|InputAxisTurnForward AxisValue) 512.0) (/ AxisValue 512.0)))

(event Input|AxisEvents|InputAxisTurnForward
  (params (AxisValue :type Float%20%28single-precision%29))
  ;[1 1 1] RightStick
  (CallFunction|StickRotatorServer (/ AxisValue 512.0) (/ (stale Input|AxisEvents|InputAxisTurnRight AxisValue) 512.0)))

(event Input|AxisEvents|InputAxisMoveRight
  (params (AxisValue :type Float%20%28single-precision%29))
  ;[1 1 1] LeftStick
  (Pawn|Input|AddMovementInput (Pawn|GetControlledPawn) "0,-90.000000,0.000000" AxisValue false))

(event Input|AxisEvents|InputAxisMoveForward
  (params (AxisValue :type Float%20%28single-precision%29))
  ;[1 1 1] LeftStick
  (Pawn|Input|AddMovementInput (Pawn|GetControlledPawn) "90.000000, 0, 0" AxisValue false))

(fn ConstructionScript)

(fn OnRepFaceRotation
  (Utilities|Casting|CastToCharacter_BP (Pawn|GetControlledPawn))
  (if (Variables|Default|GetIsFiring?)
    (Pawn|SetControlRotation (Variables|Default|GetOldRotation))
    (else
      (Pawn|SetControlRotation (Variables|Default|GetFaceRotation)))))

(fn SnapWeapon
  (bind _ascharacter_bp (Utilities|Casting|CastToCharacter_BP (Pawn|GetControlledPawn)))
  (bind _returnvalue (Game|SpawnActorfromClass "/Game/Gameplay/Weapons/Weapon_BPs/M4/M4_BP.M4_BP_C" (Transformation|GetSocketTransform (Variables|/Script/Engine.Character|GetMesh _ascharacter_bp) "skt_defaultgun" "RTS_ParentBoneSpace") "Undefined" 0 0))
  (bind _output_get (Variables|Default|SetNewVar_0 _returnvalue))
  (Transformation|AttachComponentToComponent _output_get (Variables|/Script/Engine.Character|GetMesh _ascharacter_bp) (Class|SkinnedMeshComponent|GetSocketBoneName (Variables|/Script/Engine.Character|GetMesh _ascharacter_bp) "skt_defaultgun") "KeepRelative" "KeepRelative" "KeepRelative" true)
  (Variables|/Game/Gameplay/Weapons/Weapon_BPs/General/ABP_BaseWeapon.ABP_BaseWeapon_C|SetControllerRef _output_get self))