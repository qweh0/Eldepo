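; Character Blueprint that tracks whether the character is turning left or right and passes that state to the server.
; SetTurn keeps the TurnLeft and TurnRight flags mutually exclusive, and StopTurn clears both.
; ReplicateTurn sends the flags from non-authority instances through a server set-turn event.
; RemoveWidget forwards to CallRemove, while the damage event and construction script are empty.
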(event Custom|RemoveWidget
  (Default|CallRemove))

(event Custom|StopTurn
  (params (Stop :type Boolean))
  (if Stop
    (Variables|Default|SetTurnLeft false)
    (Variables|Default|SetTurnRight false)))

(event Custom|SetTurn
  (params (LeftOrRight :type Boolean))
  (if LeftOrRight
    (Variables|Default|SetTurnLeft true)
    (Variables|Default|SetTurnRight false)
    (else
      (Variables|Default|SetTurnRight true)
      (Variables|Default|SetTurnLeft false))))

(event Custom|SRV_SetTurn
  (params (Turn%20Left :type Boolean) (Turn%20Right :type Boolean))
  (Variables|Default|SetTurnLeft Turn%20Left)
  (Variables|Default|SetTurnRight Turn%20Right))

(event Custom|ReplicateTurn
  (Networking|SwitchHasAuthority
    (:Remote
      (CallFunction|SRVSetTurn (Variables|Default|GetTurnLeft) (Variables|Default|GetTurnRight)))))

(event Game|Damage|EventAnyDamage
  (params (Damage :type Float%20%28single-precision%29) (DamageType :type Damage%20Type%20Object%20Reference) (InstigatedBy :type Controller%20Object%20Reference) (DamageCauser :type Actor%20Object%20Reference)))

(fn ConstructionScript)